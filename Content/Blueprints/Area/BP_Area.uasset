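; BP_Area is a damageable sphere zone, with radius, line thickness and label set from AreaStruct during construction.
; Player overlap runs timelines that fade its health widget in or out, calling the character's AreaDamageTimer or ClearTimerArea on every update.
; A looping one-second timer, started through PlayerDamageTimer, subtracts player Damage from area health and adds a small fraction to player health.
; At zero health, the area destroys itself and removes the widget.
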(event OnComponentBeginOverlap(Sphere)
  (params (OverlappedComponent :type Primitive%20Component%20Object%20Reference) (OtherActor :type Actor%20Object%20Reference) (OtherComp :type Primitive%20Component%20Object%20Reference) (OtherBodyIndex :type Integer) (bFromSweep :type Boolean) (SweepResult :type Hit%20Result%20Structure%20%28by%20ref%29))
  (if (Actor|ActorHasTag OtherActor "Player")
    (bind _newtrack_0 (Timeline|Timeline PlayFromStart)
      (:Update
        (Variables|/Script/UMG.Widget|SetRenderOpacity (Variables|Default|GetWBP_Healthbar) _newtrack_0)
        (bind _asbp_third_person_character (Utilities|Casting|CastToBP_ThirdPersonCharacter OtherActor))
        (bind _output_get (Variables|Default|SetAs%20BP%20Third%20Person%20Character _asbp_third_person_character))
        (Default|AreaDamageTimer _output_get)
        (Variables|/Script/UMG.TextBlock|SetText (Variables|/Game/Blueprints/widgets/WBP_HealtBarArea.WBP_HealtBarArea_C|GetTextBlock_91 (Variables|Default|GetWBP_Healthbar)) (Utilities|Text|ToText(String) (Utilities|String|Append (Utilities|String|ToString(Text) (Variables|/Script/Engine.TextRenderComponent|GetText (Variables|Default|GetTextRender))) " " (Utilities|String|ToString(Float) (Variables|/Game/Blueprints/BP_Component.BP_Component_C|GetHealth (Variables|Default|GetBP_Component))))))))))

(event OnComponentEndOverlap(Sphere)
  (params (OverlappedComponent :type Primitive%20Component%20Object%20Reference) (OtherActor :type Actor%20Object%20Reference) (OtherComp :type Primitive%20Component%20Object%20Reference) (OtherBodyIndex :type Integer))
  (if (Actor|ActorHasTag OtherActor "Player")
    (bind _newtrack_0 (Timeline|Timeline_0 PlayFromStart)
      (:Update
        (Variables|/Script/UMG.Widget|SetRenderOpacity (Variables|Default|GetWBP_Healthbar) _newtrack_0)
        (bind _asbp_third_person_character (Utilities|Casting|CastToBP_ThirdPersonCharacter OtherActor))
        (Default|ClearTimerArea _asbp_third_person_character)))))

(event EventBeginPlay
  (bind _returnvalue (UserInterface|CreateWidget "/Game/Blueprints/widgets/WBP_HealtBarArea.WBP_HealtBarArea_C"))
  (bind _output_get (Variables|Default|SetWBP_Healthbar _returnvalue))
  (UserInterface|Viewport|AddtoViewport _output_get 0)
  (Variables|/Script/UMG.Widget|SetRenderOpacity (Variables|Default|GetWBP_Healthbar) 0.0))

(fn ConstructionScript
  (bind _areastruct (Variables|Default|GetAreaStruct))
  (bind _sphere (Variables|Default|GetSphere))
  (bind (_radius _line_thickness _text) (Utilities|Struct|BreakStruct_Area _areastruct))
  (Utilities|FlowControl|Sequence
    (:then_0
      (Components|Sphere|SetSphereRadius _sphere _radius true)
      (Class|ShapeComponent|SetLineThickness _sphere _line_thickness))
    (:then_1
      (Rendering|Components|TextRender|SetText (Variables|Default|GetTextRender) _text))))

(fn TakePlayerDamage
  (bind _as_bp_third_person_character (Variables|Default|GetAs%20BP%20Third%20Person%20Character))
  (bind _bp_component (Variables|Default|GetBP_Component))
  (bind _bp_component_2 (Variables|/Game/ThirdPerson/Blueprints/BP_ThirdPersonCharacter.BP_ThirdPersonCharacter_C|GetBP_Component _as_bp_third_person_character))
  (if (<= (Variables|/Game/Blueprints/BP_Component.BP_Component_C|GetHealth _bp_component) 0.0)
    (Actor|DestroyActor)
    (Widget|RemovefromParent (Variables|Default|GetWBP_Healthbar))
    (else
      (Variables|/Game/Blueprints/BP_Component.BP_Component_C|SetHealth _bp_component (- (Variables|/Game/Blueprints/BP_Component.BP_Component_C|GetHealth _bp_component) (Variables|/Game/Blueprints/BP_Component.BP_Component_C|GetDamage (Variables|/Game/ThirdPerson/Blueprints/BP_ThirdPersonCharacter.BP_ThirdPersonCharacter_C|GetBP_Component (Variables|Default|GetAs%20BP%20Third%20Person%20Character)))))
      (Variables|/Game/Blueprints/BP_Component.BP_Component_C|SetHealth _bp_component_2 (+ (* 0.009 (Variables|/Game/Blueprints/BP_Component.BP_Component_C|GetDamage _bp_component_2)) (Variables|/Game/Blueprints/BP_Component.BP_Component_C|GetHealth _bp_component_2)))
      (Variables|/Script/UMG.TextBlock|SetText (Variables|/Game/Blueprints/widgets/WBP_HealtBarArea.WBP_HealtBarArea_C|GetTextBlock_91 (Variables|Default|GetWBP_Healthbar)) (Utilities|Text|ToText(String) (Utilities|String|Append (Utilities|String|ToString(Text) (Variables|/Script/Engine.TextRenderComponent|GetText (Variables|Default|GetTextRender))) " " (Utilities|String|ToString(Float) (Variables|/Game/Blueprints/BP_Component.BP_Component_C|GetHealth (Variables|Default|GetBP_Component)))))))))

(fn PlayerDamageTimer
  (bind _returnvalue (Utilities|Time|SetTimerbyFunctionName 0 "TakePlayerDamage" 1.0 true))
  (Variables|Default|SetPlayerTimer _returnvalue))

(fn ClearPlayerTimer
  (Utilities|Time|ClearandInvalidateTimerbyHandle (Variables|Default|GetPlayerTimer)))